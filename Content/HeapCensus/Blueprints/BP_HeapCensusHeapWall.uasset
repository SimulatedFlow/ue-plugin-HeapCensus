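; Demo wall actor that visualizes the HeapCensus demo's held UObject count as a growing grid of instanced blocks with a text caption.
; Each Tick targets one block per 20 objects up to a cap, adding a few per frame row by row and rebuilding from empty when the count drops.
; The caption shows the live count, while the construction script lays out a fixed preview grid that BeginPlay clears.
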(event `self.ReceiveBeginPlay`
  (set `self.NextY` 0.0)
  (set `self.NextZ` 35.0)
  (`InstancedStaticMeshComponent.ClearInstances` (`self.Blocks`)))

(event `self.ReceiveTick`
  (params (DeltaSeconds :type "Float (single-precision)"))
  (bind _returnvalue (`HeapCensusStatics.GetHeapCensusDemoObjectCount`))
  (bind _blocks (`self.Blocks`))
  (bind _returnvalue_2 (/ _returnvalue 20))
  (if (< _returnvalue_2 (`InstancedStaticMeshComponent.GetInstanceCount` _blocks))
    (`InstancedStaticMeshComponent.ClearInstances` _blocks)
    (set `self.NextY` 0.0)
    (set `self.NextZ` 35.0))
  (for _ (range 8)
    (if (and (< (`InstancedStaticMeshComponent.GetInstanceCount` _blocks) _returnvalue_2) (< (`InstancedStaticMeshComponent.GetInstanceCount` _blocks) 240))
      (`InstancedStaticMeshComponent.AddInstance` _blocks (`KismetMathLibrary.MakeTransform` (`KismetMathLibrary.MakeVector` 0.0 (`self.NextY`) (`self.NextZ`)) (struct) (`KismetMathLibrary.MakeVector` 0.6 0.6 0.6)) false)
      (if (>= (`self.NextY`) 1000.0)
        (set `self.NextY` 0.0)
        (set `self.NextZ` (+ (`self.NextZ`) 70.0))
        (else
          (set `self.NextY` (+ (`self.NextY`) 70.0))))))
  (`TextRenderComponent.K2_SetText` (`self.Caption`) (`KismetTextLibrary.Conv_StringToText` (`KismetStringLibrary.Concat_StrStr` "HELD UOBJECTS: " (`HeapCensusStatics.FormatCount` _returnvalue)))))

(fn `UserConstructionScript`
  (bind _blocks (`self.Blocks`))
  (`InstancedStaticMeshComponent.ClearInstances` _blocks)
  (set `self.NextY` 0.0)
  (set `self.NextZ` 35.0)
  (for _ (range 96)
    (`InstancedStaticMeshComponent.AddInstance` _blocks (`KismetMathLibrary.MakeTransform` (`KismetMathLibrary.MakeVector` 0.0 (`self.NextY`) (`self.NextZ`)) (struct) (`KismetMathLibrary.MakeVector` 0.6 0.6 0.6)) false)
    (if (>= (`self.NextY`) 1000.0)
      (set `self.NextY` 0.0)
      (set `self.NextZ` (+ (`self.NextZ`) 70.0))
      (else
        (set `self.NextY` (+ (`self.NextY`) 70.0))))))